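; BP_NPC_Base is a base NPC Blueprint for dialogue interactions, showing a character name text when the NPC is interactable.
; The construction script fills that text from CharacterName, and SetInteractableState toggles its visibility.
; ConversationClosed forwards a close message to the stored InteractInstigator, which a getter also exposes.
; Interact is empty here, and this graph never assigns InteractInstigator.
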(event `/Game/StarStray/Dialogue/Blueprints/BPI_Interactable.SetInteractableState`
  (params (`bShowInteract?` :type Boolean))
  (bind _txt_charactername (`self.Txt_CharacterName`))
  (if `bShowInteract?`
    (`SceneComponent.SetVisibility` _txt_charactername true false)
    (else
      (`SceneComponent.SetVisibility` _txt_charactername false false))))

(event `/Game/StarStray/Dialogue/Blueprints/BPI_Dialogue.ConversationClosed`
  (message `/Game/StarStray/Dialogue/Blueprints/BPI_FirstPersonCloseConversation.CloseConversation` (`self.InteractInstigator`)))

(event `/Game/StarStray/Dialogue/Blueprints/BPI_Interactable.Interact`
  (params (Intigator :type "Actor Object Reference")))

(fn `GetInteractInstigator`
  (returns (Instigator :type "Actor Object Reference"))
  (return (`self.InteractInstigator`)))

(fn `UserConstructionScript`
  (`TextRenderComponent.K2_SetText` (`self.Txt_CharacterName`) (`self.CharacterName`)))