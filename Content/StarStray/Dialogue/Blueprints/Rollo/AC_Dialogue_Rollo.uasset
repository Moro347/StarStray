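; Dialogue component for the NPC Rollo, still mostly template placeholder text around a sample quest, RolloFirstQuest.
; BeginPlay registers that quest and its stage in the journal.
; Dialogue switches on ActiveDialogueBranch, shows options gated by quest checks through UniversalChecker helpers, and changes quest state when the player answers the offer.
; The AddDialogueFast macro wraps AddDialogue, giving each of seven options its own exec output, plus a non-skippable mode without options.
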(event `self.ReceiveBeginPlay`
  (`parent.ReceiveBeginPlay`)
  (bind _journal (`self.GetJournal`))
  (`/Game/StarStray/Journal/AC_Journal.AddQuest` _journal (`self.NPCName`) "RolloFirstQuest" "info w journalu" (`|MakeArray` (make `/Game/StarStray/Journal/Struct_QuestStage` "Stage1" "info o stagu" (`|MakeMap` "wymog1" :!type "Name"))) "NewEnumerator0" 0)
  (`/Game/StarStray/Journal/AC_Journal.ChangeQuestStageRequirement` _journal "" "None" "None" false))

(fn `Dialogue`
  (`parent.Dialogue`)
  (switch `name` (`self.ActiveDialogueBranch`)
    (:`Default`
      (`self.AddDialogueFast` false "" "THIS IS NPC TEXT" "JUST WRITE IF YOU WANT THIS OPTION TO BE ALWAYS VISABLE" (`self.DialogueOptionWithUniversalChecker` "THIS DIALOGUE OPTION WILL BE VISIBLE IF THE CHECK IS TRUE" "NewEnumerator4" "RolloFirstQuest" "NewEnumerator0" "NewEnumerator5" "Stage1") (`KismetMathLibrary.SelectText` "THIS IS HOW YOU MAKE DIALOGUE OPTION WITH YOUR OWN CONDITION" "" (and (`self.UniversalChecker` "NewEnumerator3" "NAME" "NewEnumerator0" "NewEnumerator4" "NAMESTAGE") (`self.UniversalChecker` "NewEnumerator1" "NAME" "NewEnumerator0" "NewEnumerator4" "NAMESTAGE" "None" true)))
        (:`0`
          (`self.AddDialogueFast` true "" "another bubble"
            (:`Default`
              (`self.EndLine` "NewEnumerator1"))))
        (:`1`
          (`self.AddDialogueFast` false "" "kontynuujac z questem RolloFirstQuest " (`self.DialogueOptionWithUniversalChecker` "czy masz moze jakies zadanie dla mnie" "NewEnumerator0" "RolloFirstQuest") (`self.DialogueOptionWithUniversalChecker` "wracajac to tego zadania" "NewEnumerator0" "RolloFirstQuest" "NewEnumerator1") (`self.DialogueOptionWithUniversalChecker` "opowiedz mi wiecej gdzie mam tego szukac" "NewEnumerator0" "RolloFirstQuest" "NewEnumerator2")
            (:`0`
              (`self.AddDialogueFast` false "" "a mam czy chcialbys sie zajac tym i tym" "tak" "nie" :!label _label
                (:`0`
                  (`/Game/StarStray/Journal/AC_Journal.ChangeQuestState` (`self.ActiveJournal`) "NewEnumerator2" "RolloFirstQuest")
                  (`self.EndLine` "NewEnumerator1"))
                (:`1`
                  (`/Game/StarStray/Journal/AC_Journal.ChangeQuestState` (`self.ActiveJournal`) "NewEnumerator1" "RolloFirstQuest")
                  (`self.EndLine` "NewEnumerator1"))))
            (:`1`
              (goto _label))
            (:`2`
              (`self.EndLine` "NewEnumerator1"))))
        (:`2`
          (set `self.ActiveDialogueBranch` "YOURBRANCH")
          (`self.EndLine` "NewEnumerator2"))))
    (:`YOURBRANCH`
      (`self.AddDialogueFast` false "" "BRANCHES ARE EASIEST WAY TO CONTAIN QUESTS" "CONTINUE WITH QUEST" "END QUEST"
        (:`0`
          (`self.AddDialogueFast` false "" "NPC GENERIC TEXT" "CONDITION" "YOUR" "QUEST" "WITH" "PLAYER" "DIALOGUE" "OPTIONS"))
        (:`1`
          (set `self.ActiveDialogueBranch` "None")
          (`self.EndLine` "NewEnumerator1"))))))