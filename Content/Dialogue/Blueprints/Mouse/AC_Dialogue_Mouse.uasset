(fn `Dialogue`
  (`parent.Dialogue`)
  (switch `name` (`self.ActiveDialogueBranch`)
    (:`Default`
      (bind (_state _optionindex) (`self.AddDialogue` "Mouse" "Hi, do you have any cheese?" (`|MakeArray` "yes" "no" :!type "Text")))
      (switch `/Game/Dialogue/DialogueSystemComponents/Enum_DialogueState` _state
        (:`NewEnumerator0`
          (switch `int` _optionindex
            (:`0`
              (bind (_state_2 _optionindex_2) (`self.AddDialogue` "Mouse" "Ahh, thats great, can i have some?" (`|MakeArray` "give cheese" "keep cheese" :!type "Text")))
              (switch `/Game/Dialogue/DialogueSystemComponents/Enum_DialogueState` _state_2
                (:`NewEnumerator0`
                  (switch `int` _optionindex_2
                    (:`0`
                      (bind _state_3 (`self.AddDialogue` "Mouse" "Thank you, you are so kind" (`|MakeArray`)))
                      (switch `/Game/Dialogue/DialogueSystemComponents/Enum_DialogueState` _state_3
                        (:`NewEnumerator0`
                          (`self.SetDialogueBranch` "GivenCheese")
                          (`self.CloseConversation`))))
                    (:`1`
                      (bind _state_4 (`self.AddDialogue` "Mouse" "You big meany!" (`|MakeArray`)))
                      (switch `/Game/Dialogue/DialogueSystemComponents/Enum_DialogueState` _state_4
                        (:`NewEnumerator0`
                          (`self.RemoveDialogueProgress` 2)
                          (`self.CloseConversation`))))))))
            (:`1`
              (bind _state_5 (`self.AddDialogue` "Mouse" "Aww... thats a shame, i really want some cheese" (`|MakeArray`)))
              (switch `/Game/Dialogue/DialogueSystemComponents/Enum_DialogueState` _state_5
                (:`NewEnumerator0`
                  (`self.ClearDialogueProgress`)
                  (`self.CloseConversation`))))))))
    (:`GivenCheese`
      (bind _state_6 (`self.AddDialogue` "Mouse" (select `int` (`KismetMathLibrary.RandomIntegerInRange` 0 1) :`0` "You are such a nice person!" :`1` "nomm nomm nomm" :!type "Text") (`|MakeArray` "continue" :!type "Text")))
      (switch `/Game/Dialogue/DialogueSystemComponents/Enum_DialogueState` _state_6
        (:`NewEnumerator0`
          (`self.ClearDialogueProgress`)
          (`self.CloseConversation`))))))