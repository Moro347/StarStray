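; Dialogue trigger component that serves as an example template for triggered dialogue, with placeholder lines and a sample branch.
; The Dialogue override calls its parent, flags AlreadyTalking, then chains lines through Updated and Default outputs.
; A sample boolean picks between two branches, which both clear the flag and end the line.
; The AddDialogueFast macro wraps AddDialogue, varying its options and audio/animation inputs by the NotSkipable flag.
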(event `self.ReceiveBeginPlay`
  (`parent.ReceiveBeginPlay`))

(fn `Dialogue`
  (`parent.Dialogue`)
  (set `self.AlreadyTalking` true)
  (switch `name` (`self.ActiveDialogueBranch`)
    (:`Default`
      (`self.AddDialogueFast` true "" "This is Dialogue that had been triggrered"
        (:`Updated`
          (`KismetSystemLibrary.PrintText` "here you should place stuff that should happen immidietly after triggering it"))
        (:`Default`
          (`self.AddDialogueFast` true "" "that is how you should continue it"
            (:`Default`
              (if (`self.ThisCanBeAJournalValue`)
                (`self.AddDialogueFast` true "" "if you want branches"
                  (:`Default`
                    _))
                (else
                  (`self.AddDialogueFast` true "" "here branch nr2"
                    (:`Default`
                      _))))
              (set `self.AlreadyTalking` false)
              (`self.EndLine` "NewEnumerator1"))))))))