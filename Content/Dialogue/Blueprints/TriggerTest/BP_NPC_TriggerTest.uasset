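; BP_NPC_TriggerTest is a test NPC that starts dialogue when an actor enters its box trigger, with an empty Interact event.
; BeginPlay passes CharacterName to the ACDialogueTrigger component, then runs the parent logic.
; On overlap, actors implementing BPI_JournalHandler are stored as InteractInstigator.
; If no conversation is running, it opens one, hides the mouse cursor and sets game-only input.
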(event `self.ReceiveBeginPlay`
  (set `/Game/Dialogue/DialogueSystemComponents/AC_Dialogue_Base.NPCName` (`self.CharacterName`) (`self.AC_Dialogue_Trigger`))
  (`parent.ReceiveBeginPlay`))

(event `/Game/Dialogue/Blueprints/BPI_Interactable.Interact`
  (params (Intigator :type "Actor Object Reference")))

(event `self.Box.OnComponentBeginOverlap`
  (params (OverlappedComponent :type "PrimitiveComponent Object Reference") (OtherActor :type "Actor Object Reference") (OtherComp :type "PrimitiveComponent Object Reference") (OtherBodyIndex :type Integer) (bFromSweep :type Boolean) (SweepResult :type "HitResult Structure (by ref)"))
  (bind _returnvalue (`GameplayStatics.GetPlayerController` 0))
  (if (`KismetSystemLibrary.DoesImplementInterface` OtherActor "/Game/Journal/BPI_JournalHandler.BPI_JournalHandler_C")
    (set `self.InteractInstigator` OtherActor)
    (if (not (`/Game/Dialogue/Blueprints/TriggerTest/AC_Dialogue_Trigger.AlreadyTalking` (`self.AC_Dialogue_Trigger`)))
      (`/Game/Dialogue/DialogueSystemComponents/AC_Dialogue_Base.OpenConversation` (`self.AC_Dialogue_Trigger`))
      (set `PlayerController.bShowMouseCursor` false _returnvalue)
      (`WidgetBlueprintLibrary.SetInputMode_GameOnly` _returnvalue))))

(fn `GetInteractInstigator`
  (returns (Instigator :type "Actor Object Reference"))
  (return null))

(fn `UserConstructionScript`
  (`parent.UserConstructionScript`))