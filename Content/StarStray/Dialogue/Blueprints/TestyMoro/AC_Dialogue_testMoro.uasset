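; Dialogue component for a test NPC, a Polish-speaking wood trader who offers a quest to bring ten pieces of wood.
; BeginPlay registers QuestS in the journal; Dialogue switches on ActiveDialogueBranch between greeting, backstory and quest talk.
; Quest options are filtered by quest state and can accept, refuse or complete it through the journal.
; The AddDialogueFast macro routes chosen options to exec pins; leftover template examples and alternative state-based branching are unconnected.
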(event `self.ReceiveBeginPlay`
  (`parent.ReceiveBeginPlay`)
  (bind _journal (`self.GetJournal`))
  (`/Game/StarStray/Journal/AC_Journal.AddQuest` _journal (`self.NPCName`) "QuestS" "" (`|MakeArray` (make `/Game/StarStray/Journal/Struct_QuestStage` "Drewno" "" (`|MakeMap` "10 Drewna" :!type "Name"))) "NewEnumerator1" 0))

(fn `Dialogue`
  (`parent.Dialogue`)
  ;[1 1 1] You can choose Active Branch here(can be any number of branches, including 0)
  (switch `name` (`self.ActiveDialogueBranch`)
    (:`Default`
      (`self.AddDialogueFast` true "" (select `int` (`KismetMathLibrary.RandomIntegerInRange` 0 3) :`0` "Witaj" :`1` "Czego chcesz" :`2` "Noo.." :`3` "O kolejny kmiot" :!type "Text")
        (:`Default`
          (`self.AddDialogueFast` false "" "W czym moge pomóc?" "Opowiedz mi o sobie" (`self.DialogueOptionWithUniversalChecker` "Słyszałem, że masz cos dla mnie do roboty" "NewEnumerator0" "QuestS" "NewEnumerator1") "Żegnaj"
            (:`0`
              (set `self.ActiveDialogueBranch` "Opowiedz")
              (`self.EndLine` "NewEnumerator2"))
            (:`1`
              (set `self.ActiveDialogueBranch` "MisjaDrewno")
              (`self.EndLine` "NewEnumerator2"))
            (:`2`
              (`self.EndLine` "NewEnumerator1" 1))))))
    (:`Opowiedz`
      (`self.AddDialogueFast` true "" "Pochodze z małej wioski. Jestem sierotą i handluję drewnem"
        (:`Default`
          (set `self.ActiveDialogueBranch` "None")
          (`self.EndLine` "NewEnumerator2"))))
    (:`MisjaDrewno`
      (`self.AddDialogueFast` false "" (select `int` (`KismetMathLibrary.RandomIntegerInRange` 0 2) :`0` "Muszę wracać do pracy" :`1` "Wybacz, nie mam teraz czasu" :`2` "Przepraszam przyjacielu, na mnie już czas" :!type "Text") (`self.DialogueOptionWithUniversalChecker` "Widzę, że brakuje Ci drewna" "NewEnumerator0" "QuestS" "NewEnumerator1") (`self.DialogueOptionWithUniversalChecker` "Gdzię znajdę drewno?" "NewEnumerator0" "QuestS" "NewEnumerator2") (`self.DialogueOptionWithUniversalChecker` "Przyniosłem drewno" "NewEnumerator0" "QuestS" "NewEnumerator5" "NewEnumerator4" "Drewno" "10 Drewna")
        (:`0`
          (`self.AddDialogueFast` false "" "Potrzebuje pomocy w tartaku" "Terac nie mam czasu" "Czego konkretnie potrzebujesz" "Poszukaj sobie kogos innego"
            (:`0`
              (`self.EndLine` "NewEnumerator3" 2))
            (:`1`
              (`self.AddDialogueFast` false "" "Potrzebuję 10 sztuk drewna. Dziękuję za pomoc" "Robi się"
                (:`0`
                  (`/Game/StarStray/Journal/AC_Journal.ChangeQuestState` (`self.ActiveJournal`) "NewEnumerator2" "QuestS")
                  (`self.EndLine` "NewEnumerator1"))))
            (:`2`
              (`self.AddDialogueFast` false "" "Jesstes pewnien przyjacielu?" "Tak, spieprzaj dziadu" "Zastanowie sie"
                (:`0`
                  (`/Game/StarStray/Journal/AC_Journal.ChangeQuestState` (`self.ActiveJournal`) "NewEnumerator4" "QuestS")
                  (`self.EndLine` "NewEnumerator1"))
                (:`1`
                  (`self.EndLine` "NewEnumerator3" 2))))))
        (:`1`
          (`self.AddDialogueFast` false "" "Idź nad strumień, rosną tam nejlepsze modrzewie w okolicy." "Już zabieram się do pracy"
            (:`0`
              (`self.EndLine` "NewEnumerator1"))))
        (:`2`
          (`self.AddDialogueFast` false "" "Bardzo Ci dziękuję" "Polecam się"
            (:`0`
              (`/Game/StarStray/Journal/AC_Journal.ChangeQuestState` (`self.ActiveJournal`) "NewEnumerator3" "QuestS")
              (set `self.ActiveDialogueBranch` "None")
              (`self.EndLine` "NewEnumerator1"))))))))