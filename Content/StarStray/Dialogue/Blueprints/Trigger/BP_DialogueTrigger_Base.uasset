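; Base trigger volume that starts a dialogue when an actor implementing BPI_JournalHandler overlaps its box.
; It stores that actor as the instigator, sets a running guard and calls OpenConversationChildSetup, an empty hook for child Blueprints.
; OpenConversationEvent opens the conversation on the object passed to it.
; ConversationClosed notifies the instigator and clears the guard only if Repeatable, so other triggers fire once.
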(event `self.Box.OnComponentBeginOverlap`
  (params (OverlappedComponent :type "PrimitiveComponent Object Reference") (OtherActor :type "Actor Object Reference") (OtherComp :type "PrimitiveComponent Object Reference") (OtherBodyIndex :type Integer) (bFromSweep :type Boolean) (SweepResult :type "HitResult Structure (by ref)"))
  (if (`KismetSystemLibrary.DoesImplementInterface` OtherActor "/Game/StarStray/Journal/BPI_JournalHandler.BPI_JournalHandler_C")
    (set `self.InteractInstigator` OtherActor)
    (if (not (`self.DialogueRunning`))
      (set `self.DialogueRunning` true)
      (`self.OpenConversationChildSetup`))))

(event `OpenConversationEvent`
  (params (NewParam :type "/Game/StarStray/Dialogue/DialogueSystemComponents/AC_Dialogue_Base Object Reference"))
  (`/Game/StarStray/Dialogue/DialogueSystemComponents/AC_Dialogue_Base.OpenConversation` NewParam false))

(event `OpenConversationChildSetup`)

(event `/Game/StarStray/Dialogue/Blueprints/BPI_Dialogue.ConversationClosed`
  (message `/Game/StarStray/Dialogue/Blueprints/BPI_FirstPersonCloseConversation.CloseConversation` (`self.InteractInstigator`))
  (if (`self.Repeatable`)
    (set `self.DialogueRunning` false)))

(fn `UserConstructionScript`)