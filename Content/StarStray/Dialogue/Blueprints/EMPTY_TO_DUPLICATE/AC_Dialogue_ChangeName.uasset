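; Template NPC dialogue component, meant to be duplicated and renamed, with placeholder lines showing how to author conversations in StarStray.
; The Dialogue override switches on ActiveDialogueBranch, with options changing or clearing the branch to contain quests and ending lines through EndLine.
; UniversalChecker quest checks control option visibility, either through a helper or custom SelectText conditions.
; The AddDialogueFast macro wraps AddDialogue, routing up to seven options to separate outputs and supporting non-skippable bubbles.
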(fn `Dialogue`
  (`parent.Dialogue`)
  (switch `name` (`self.ActiveDialogueBranch`)
    (:`Default`
      (`self.AddDialogueFast` false "" "THIS IS NPC TEXT" "JUST WRITE IF YOU WANT THIS OPTION TO BE ALWAYS VISABLE" (`self.DialogueOptionWithUniversalChecker` "THIS DIALOGUE OPTION WILL BE VISIBLE IF THE CHECK IS TRUE") (`KismetMathLibrary.SelectText` "THIS IS HOW YOU MAKE DIALOGUE OPTION WITH YOUR OWN CONDITION" "" (and (`self.UniversalChecker` "NewEnumerator3" "NAME" "NewEnumerator0" "NewEnumerator4" "NAMESTAGE") (`self.UniversalChecker` "NewEnumerator1" "NAME" "NewEnumerator0" "NewEnumerator4" "NAMESTAGE" "None" true)))
        (:`0`
          (`self.AddDialogueFast` true "" "another bubble"
            (:`Default`
              (`self.EndLine` "NewEnumerator1"))))
        (:`1`
          (`self.EndLine` "NewEnumerator1"))
        (:`2`
          (set `self.ActiveDialogueBranch` "YOURBRANCH")
          (`self.EndLine` "NewEnumerator2"))))
    (:`YOURBRANCH`
      (`self.AddDialogueFast` false "" "BRANCHES ARE EASIEST WAY TO CONTAIN QUESTS" "CONTINUE WITH QUEST" "END QUEST"
        (:`0`
          (`self.AddDialogueFast` false "" "NPC GENERIC TEXT" "CONDITION" "YOUR" "QUEST" "WITH" "PLAYER" "DIALOGUE" "OPTIONS"))
        (:`1`
          (set `self.ActiveDialogueBranch` "None")
          (`self.EndLine` "NewEnumerator1"))))))