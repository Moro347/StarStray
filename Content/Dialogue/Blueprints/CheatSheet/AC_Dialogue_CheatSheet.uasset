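; Example NPC dialogue component that serves as a cheat sheet for building branching, quest-driven conversations.
; BeginPlay registers a two-stage Quest1 in the journal.
; Dialogue switches on the active branch and nests lines whose checker-gated options change quest state, requirements, stages or branch, with EndLine closing or stepping back.
; The AddDialogueFast macro wraps AddDialogue, routing the chosen option to exec pins, with an option-less NotSkipable mode.
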(event `self.ReceiveBeginPlay`
  (`parent.ReceiveBeginPlay`)
  (bind _journal (`self.GetJournal`))
  (`/Game/Journal/AC_Journal.AddQuest` _journal (`self.NPCName`) "Quest1" "" (`|MakeArray` (make `/Game/Journal/Struct_QuestStage` "Stage1" "" (`|MakeMap` "Req1" :!type "Name")) (make `/Game/Journal/Struct_QuestStage` "Stage2" "" (`|MakeMap` "Req1" false "Req2" :!type "Name"))) "NewEnumerator0" 0))

(fn `Dialogue`
  (`parent.Dialogue`)
  ;[1 1 1] You can choose Active Branch here(can be any number of branches, including 0)
  (switch `name` (`self.ActiveDialogueBranch`)
    (:`Default`
      (`self.AddDialogueFast` false "" "Hi i am Cheat, what do you want to do?" (`self.DialogueOptionWithUniversalChecker` "Set My Quest1 To Availble" "NewEnumerator0" "Quest1") (`self.DialogueOptionWithUniversalChecker` "Let's continue with Quest1" "NewEnumerator4" "Quest1" "NewEnumerator1" "NewEnumerator5") "As you can see you can put everything from one quest into 1 option to organize you dialogue better" "Bye"
        (:`0`
          ;[0.6569 1 0.274] you dont have to change availibility in dialogue, you can do it anywhere anyhow
          (`self.AddDialogueFast` false "" "Now you can set Quest1 to availble or not" "Yes" "Don't"
            (:`0`
              (`/Game/Journal/AC_Journal.ChangeQuestState` (`self.ActiveJournal`) "NewEnumerator1" "Quest1")
              (`self.EndLine` "NewEnumerator2"))
            (:`1`
              (`self.EndLine` "NewEnumerator1"))))
        (:`1`
          (`self.AddDialogueFast` false "" "Something With Quest1" (`self.DialogueOptionWithUniversalChecker` "i want to set Quest1 State  to InProgress" "NewEnumerator0" "Quest1" "NewEnumerator1") (`self.DialogueOptionWithUniversalChecker` "Let's continue with Quest1" "NewEnumerator0" "Quest1" "NewEnumerator2") (`self.DialogueOptionWithUniversalChecker` "I have done everything you asked for" "NewEnumerator0" "Quest1" "NewEnumerator5") "Bye"
            (:`0`
              (`self.AddDialogueFast` false "" "Do You A Mighty Accept This Mission ?" "Yeah whatever.." "FUCK NO"
                (:`0`
                  (`/Game/Journal/AC_Journal.ChangeQuestState` (`self.ActiveJournal`) "NewEnumerator2" "Quest1")
                  (`self.EndLine` "NewEnumerator1" 2))
                (:`1`
                  ;[0.7659 0.238 1] Changing active branch
                  (`/Game/Journal/AC_Journal.ChangeQuestState` (`self.ActiveJournal`) "NewEnumerator4" "Quest1")
                  (set `self.ActiveDialogueBranch` "Quest1Failure")
                  (`self.EndLine` "NewEnumerator1" 2))))
            (:`1`
              (`self.AddDialogueFast` false "" "Here you can go through your stages" (`self.DialogueOptionWithUniversalChecker` "Lets talk about first stage" "NewEnumerator3" "Quest1" "NewEnumerator0" "NewEnumerator4" "Stage1") (`self.DialogueOptionWithUniversalChecker` "Lets talk about second stage" "NewEnumerator3" "Quest1" "NewEnumerator0" "NewEnumerator4" "Stage2") "bye"
                (:`0`
                  ;[1 0.7706 0.3362] How to change what NPC says
                  (if (`/Game/Journal/AC_Journal.GetQuestStageRequirementS` (`self.ActiveJournal`) "Quest1" "Stage1")
                    ;;[1 1 1] Comment
                    (`self.AddDialogueFast` false "" "here lets progress stage" "ok"
                      (:`0`
                        (`/Game/Journal/AC_Journal.ProgressQuestStage` (`self.ActiveJournal`) "Quest1" "Stage1" false)
                        (`self.EndLine` "NewEnumerator1" 2)))
                    (else
                      (`self.AddDialogueFast` false "" "here lets just change the requirement of stage1 to true" "ok"
                        (:`0`
                          (`/Game/Journal/AC_Journal.ChangeQuestStageRequirement` (`self.ActiveJournal`) "Quest1" "Stage1" "Req1" true)
                          (`self.EndLine` "NewEnumerator1" 2))))))
                (:`1`
                  ;[1 0.7379 0.305] Reverse Logic
                  (`self.AddDialogueFast` false "" "Have you done what i asked you?" (`self.DialogueOptionWithUniversalChecker` "Yes" "NewEnumerator1" "Quest1" "NewEnumerator0" "NewEnumerator4" "Stage2") (`self.DialogueOptionWithUniversalChecker` "No" "NewEnumerator1" "Quest1" "NewEnumerator0" "NewEnumerator4" "Stage2" "None" true)
                    (:`0`
                      ;;[1 1 1] this should change quest1 to state met all conditions
                      (`/Game/Journal/AC_Journal.ProgressQuestStage` (`self.ActiveJournal`) "Quest1" "Stage2" false)
                      (`self.EndLine` "NewEnumerator1"))
                    (:`1`
                      (`self.EndLine` "NewEnumerator1"))))
                (:`2`
                  (`self.EndLine` "NewEnumerator1"))))
            (:`2`
              (`self.AddDialogueFast` false "" "meyby reward here?" "thank you" "not yet"
                (:`0`
                  ;[0.9668 0.5747 1] another place you can use active branch
                  (`/Game/Journal/AC_Journal.ChangeQuestState` (`self.ActiveJournal`) "NewEnumerator3" "Quest1")
                  (set `self.ActiveDialogueBranch` "ShowMeRandom")
                  (`self.EndLine` "NewEnumerator1"))
                (:`1`
                  (`self.EndLine` "NewEnumerator1"))))
            (:`3`
              (`self.EndLine` "NewEnumerator1"))))
        (:`2`
          ;[1 0.8195 0.3247] Two types of ending lines. and bubble without options to choose
          (`self.AddDialogueFast` false "" "this will clear conversation progress and close it" "ok"
            (:`Updated`
              (`KismetSystemLibrary.PrintText` "this should appear immediately after creating this conversation bubble"))
            (:`0`
              (`self.EndLine` "NewEnumerator1"))))
        (:`3`
          (`self.AddDialogueFast` true "" "this will clear conversation progress and won't close it" "THIS" "DONT" "MATTER" "IF" "NOTSKIPABLE" "IS" "CHECKED"
            (:`Updated`
              (`KismetSystemLibrary.PrintText` "this should appear immediately after creating this conversation bubble"))
            (:`Default`
              (`self.EndLine` "NewEnumerator2"))))))
    (:`Quest1Failure`
      ;[0.7814 0.2419 1] How to use active branch, you can make it "unescapable" stick to only this branch, or create new branch or just get back to default
      (`self.AddDialogueFast` false "" "You can have your \"player has consequences here\"" "ok"
        (:`0`
          (set `self.ActiveDialogueBranch` "Default")
          (`self.EndLine` "NewEnumerator2"))))
    (:`ShowMeRandom`
      (`self.AddDialogueFast` false "" (select `int` (`KismetMathLibrary.RandomIntegerInRange` 0 2) :`0` "oyyoyoyo" :`1` "Buuuurp" :`2` "no hejka" :!type "Text") "ok" "tell me something different"
        (:`0`
          (set `self.ActiveDialogueBranch` "Default")
          (`self.EndLine` "NewEnumerator2"))
        (:`1`
          (`self.EndLine` "NewEnumerator0" 1))))))