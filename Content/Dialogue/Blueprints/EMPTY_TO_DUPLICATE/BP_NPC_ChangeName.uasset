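; BP_NPC_ChangeName is a template NPC Blueprint, kept in a folder of assets to duplicate, that the player can interact with to start dialogue.
; On BeginPlay it passes its CharacterName to the ACDialogueChangeName component as the NPC name.
; Its Interact event stores the instigator in InteractInstigator, then tells that component to open the conversation.
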(event `self.ReceiveBeginPlay`
  (set `/Game/Dialogue/DialogueSystemComponents/AC_Dialogue_Base.NPCName` (`self.CharacterName`) (`self.AC_Dialogue_ChangeName`))
  (`parent.ReceiveBeginPlay`))

(event `/Game/Dialogue/Blueprints/BPI_Interactable.Interact`
  (params (Intigator :type "Actor Object Reference"))
  (set `self.InteractInstigator` Intigator)
  (`/Game/Dialogue/DialogueSystemComponents/AC_Dialogue_Base.OpenConversation` (`self.AC_Dialogue_ChangeName`)))

(fn `UserConstructionScript`
  (`parent.UserConstructionScript`))