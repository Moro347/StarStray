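; Test NPC dialogue component for StarStray, extending a parent dialogue component with a short placeholder conversation.
; On BeginPlay it registers a quest with an empty placeholder stage in the journal under the NPC's name.
; The Dialogue override switches on the active branch and chains AddDialogueFast calls to EndLine.
; That macro wraps AddDialogue, showing either an option-less line or up to ten choices routed by selected index, depending on Condition.
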(event `self.ReceiveBeginPlay`
  (`parent.ReceiveBeginPlay`)
  (bind _journal (`self.GetJournal`))
  (`/Game/StarStray/Journal/AC_Journal.AddQuest` _journal (`self.NPCName`) "" "" (`|MakeArray` (make `/Game/StarStray/Journal/Struct_QuestStage` "None" "" (`|MakeMap` "None" :!type "Name"))) "NewEnumerator0" 0))

(fn `Dialogue`
  (`parent.Dialogue`)
  (switch `name` (`self.ActiveDialogueBranch`)
    (:`Default`
      (`self.AddDialogueFast` true "" "123"
        (:`Default`
          (`self.AddDialogueFast` false "" "cos tam mowi" "opcja 0"
            (:`0`
              (`self.AddDialogueFast` false "" "opcja 0 zadzialala" "ok"
                (:`0`
                  (`self.EndLine` "NewEnumerator1"))))))))))